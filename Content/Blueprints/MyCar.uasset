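; MyCar is a car Blueprint whose only graph logic is an elapsed-time counter in minutes and seconds.
; Tick feeds a one-second Delay, which ignores re-triggers while pending, so TimeSec increments roughly once per second rather than every frame.
; When TimeSec passes 59, it resets to zero and TimeMin increments.
; The construction script is empty, and no driving logic appears in these graphs.
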(event EventTick
  (params (DeltaSeconds :type Float%20%28single-precision%29))
  ;[1 1 1] Timer
  (Utilities|FlowControl|Delay 1.0)
  (Variables|Default|SetTimeSec (+ (Variables|Default|GetTimeSec) 1))
  (if (> (Variables|Default|GetTimeSec) 59)
    (Variables|Default|SetTimeMin (+ (Variables|Default|GetTimeMin) 1))
    (Variables|Default|SetTimeSec 0)))

(fn ConstructionScript)