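; Electric hazard-style actor that spawns an electric ball and keeps it wandering randomly within an area marked by two cylinders.
; On BeginPlay it reads both cylinder positions as opposite XY bounds and spawns the ball at a random point between them at fixed height.
; BallMove and ElectricBallMoving call each other in a loop, picking a new random target and gliding the ball's root there with MoveComponentTo.
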(event Custom|Electric%20ball%20moving
  (params (INdex :type Integer))
  (if (Variables|Default|GetElectricBall%20Exist)
    (Components|MoveComponentTo (Variables|/Script/Engine.Actor|GetRootComponent (Variables|Default|GetBall1)) (Variables|Default|GetSpawn%20Ele) "0, 0, 0" false false 5.0 false)
    (CallFunction|BallMove)))

(event Custom|ball%20move
  (params (Loc%20move%20index :type Integer))
  (bind _newparam (CallFunction|BallSpawnandTransform (Variables|Default|GetLocation) (Variables|Default|GetLocation%202)))
  (Variables|Default|SetSpawn%20Ele _newparam)
  (CallFunction|ElectricBallMoving))

(event EventBeginPlay
  (bind _output_get (Variables|Default|SetLocation (Transformation|GetWorldLocation (Variables|Default|GetCylinder))))
  (bind _output_get_2 (Variables|Default|SetLocation%202 (Transformation|GetWorldLocation (Variables|Default|GetCylinder2))))
  (bind _newparam (CallFunction|BallSpawnandTransform _output_get _output_get_2))
  (bind _output_get_3 (Variables|Default|SetSpawn%20Ele _newparam))
  (bind _returnvalue (Game|SpawnActorfromClass "/Game/Blueprints/electricBallBlueprint.electricBallBlueprint_C" (Math|Conversions|ToTransform(Vector) _output_get_3) "Undefined" 0 0))
  (Variables|Default|SetBall1 _returnvalue)
  (Variables|Default|SetElectricBall%20Exist true)
  (bind _output_get_4 (Variables|Default|SetLocation (Transformation|GetWorldLocation (Variables|Default|GetCylinder))))
  (bind _output_get_5 (Variables|Default|SetLocation%202 (Transformation|GetWorldLocation (Variables|Default|GetCylinder2))))
  (bind _newparam_2 (CallFunction|BallSpawnandTransform _output_get_4 _output_get_5))
  (Variables|Default|SetSpawn%20Ele _newparam_2)
  (CallFunction|ElectricBallMoving))

(fn ConstructionScript)

(fn BallSpawnandTransform
  (params (Loc :type Vector) (Loc2 :type Vector))
  (bind _output_get (Variables|Default|SetMax%20X (.x Loc)))
  (bind _output_get_2 (Variables|Default|SetMax%20Y (.y Loc)))
  (bind _output_get_3 (Variables|Default|SetMin%20X (.x Loc2)))
  (bind _output_get_4 (Variables|Default|SetMin%20Y (.y Loc2)))
  (return (Math|Vector|MakeVector (Math|Random|RandomFloatinRange _output_get_3 _output_get) (Math|Random|RandomFloatinRange _output_get_4 _output_get_2) 9e+01)))