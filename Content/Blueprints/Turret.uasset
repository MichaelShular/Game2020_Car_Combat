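; Enemy turret actor that tracks the player within attack range and fires bullets from two barrels.
; Each tick it interpolates the barrels' pitch and yaw toward the player when in range, updates the range flag by distance, and destroys itself at zero health.
; A self-calling retriggerable-delay loop started on BeginPlay spawns BP_Bullet at both barrel sockets while in range.
; Aim interpolation uses a constant delta time, so turn speed depends on frame rate.
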(event Custom|TurretRotation
  (bind _returnvalue (Game|Player|GetPlayerPawn 0))
  (bind _barrels (Variables|Default|GetBarrels))
  (bind _returnvalue_2 (Transformation|GetWorldLocation _barrels))
  (bind _returnvalue_3 (Pawn|GetNavAgentLocation _returnvalue))
  (bind _returnvalue_4 (Math|Rotator|FindLookatRotation _returnvalue_2 _returnvalue_3))
  (bind (_roll _pitch _yaw) (Math|Rotator|BreakRotator _returnvalue_4))
  ;[1 1 1] Auto Targeting
  (if (Variables|Default|GetInRange)
    (Transformation|SetWorldRotation (Variables|Default|GetBarrels) (Math|Interpolation|RInterpTo (Transformation|GetWorldRotation (Variables|Default|GetBarrels)) (Math|Rotator|MakeRotator 0.0 _pitch _yaw) (Variables|Default|GetDeltaTime) (Variables|Default|GetRoationSpeed)) false false)))

(event Custom|AggroRange
  (if (< (Transformation|GetDistanceTo self (Game|Player|GetPlayerPawn 0)) (Variables|Default|GetAttackRange))
    (Variables|Default|SetInRange true)
    (else
      (Variables|Default|SetInRange false))))

(event Custom|Shooting
  (if (Variables|Default|GetInRange)
    (Game|SpawnActorfromClass "/Game/Blueprints/BP_Bullet.BP_Bullet_C" (Transformation|GetSocketTransform (Variables|Default|GetBarrels) "Barrel_1" "RTS_World") "Undefined" 0 0)
    (Game|SpawnActorfromClass "/Game/Blueprints/BP_Bullet.BP_Bullet_C" (Transformation|GetSocketTransform (Variables|Default|GetBarrels) "Barrel_2" "RTS_World") "Undefined" 0 0)
    (Utilities|FlowControl|RetriggerableDelay (Variables|Default|GetFireRate))
    (CallFunction|Shooting)
    (else
      (Utilities|FlowControl|RetriggerableDelay (Variables|Default|GetFireRate))
      (CallFunction|Shooting))))

(event EventBeginPlay
  (CallFunction|Shooting))

(event EventTick
  (params (DeltaSeconds :type Float%20%28single-precision%29))
  (Variables|Default|SetDeltaTime 1.0)
  (CallFunction|TurretRotation)
  (CallFunction|AggroRange)
  (if (<= (Variables|Default|GetT_Health) 0)
    (Actor|DestroyActor)))

(fn ConstructionScript)