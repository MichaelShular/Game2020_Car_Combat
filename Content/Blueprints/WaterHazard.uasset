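; WaterHazard is a hazard actor that penalizes the player's wheeled vehicle for entering water.
; When its Box begins an overlap while WaterOn is true, it casts the other actor to MyWheeledVehicleBlueprint.
; It then subtracts WaterDamage from PHealth, zeroes the mesh's physics linear velocity, and teleports the vehicle to its stored MoveLocation.
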(event OnComponentBeginOverlap(Box)
  (params (OverlappedComponent :type Primitive%20Component%20Object%20Reference) (OtherActor :type Actor%20Object%20Reference) (OtherComp :type Primitive%20Component%20Object%20Reference) (OtherBodyIndex :type Integer) (bFromSweep :type Boolean) (SweepResult :type Hit%20Result%20Structure%20%28by%20ref%29))
  (if (Variables|Default|GetWater%20on)
    (bind _asmy_wheeled_vehicle_blueprint (Utilities|Casting|CastToMyWheeledVehicleBlueprint OtherActor))
    (Variables|/Game/Player/MyWheeledVehicleBlueprint.MyWheeledVehicleBlueprint_C|SetP_Health _asmy_wheeled_vehicle_blueprint (- (Variables|/Game/Player/MyWheeledVehicleBlueprint.MyWheeledVehicleBlueprint_C|GetP_Health _asmy_wheeled_vehicle_blueprint) (Variables|Default|GetWater%20damage)))
    (Physics|SetPhysicsLinearVelocity (Variables|/Script/PhysXVehicles.WheeledVehicle|GetMesh _asmy_wheeled_vehicle_blueprint) "0, 0, 0" false "None")
    (Transformation|SetWorldLocation (Variables|/Script/Engine.Actor|GetRootComponent _asmy_wheeled_vehicle_blueprint) (Variables|/Game/Player/MyWheeledVehicleBlueprint.MyWheeledVehicleBlueprint_C|GetMove%20location _asmy_wheeled_vehicle_blueprint) false true)))

(event EventBeginPlay)

(event Collision|EventActorBeginOverlap
  (params (OtherActor :type Actor%20Object%20Reference)))

(event EventTick
  (params (DeltaSeconds :type Float%20%28single-precision%29)))

(fn ConstructionScript)