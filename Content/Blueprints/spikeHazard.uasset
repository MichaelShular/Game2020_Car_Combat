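; Spike hazard actor that repeatedly moves four cone meshes in a smash motion, starting at BeginPlay.
; Smash starts four one-second MoveComponentTo moves at once, then re-calls itself after the last finishes and a short random delay.
; MoveDown builds each target by negating the bounds origin Z while keeping relative X and Y.
; A MoveUp counterpart is defined but never called.
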(event Custom|Smash
  (bind _cone (Variables|Default|GetCone))
  (bind _cone1 (Variables|Default|GetCone1))
  (bind _cone3 (Variables|Default|GetCone3))
  (bind _cone2 (Variables|Default|GetCone2))
  (Utilities|FlowControl|Sequence
    (:then_0
      (bind _newpos (CallFunction|MoveDown _cone))
      (Components|MoveComponentTo _cone _newpos "0, 0, 0" false false 1.0 false))
    (:then_1
      (bind _newpos_2 (CallFunction|MoveDown _cone1))
      (Components|MoveComponentTo _cone1 _newpos_2 "0, 0, 0" false false 1.0 false))
    (:then_2
      (bind _newpos_3 (CallFunction|MoveDown _cone2))
      (Components|MoveComponentTo _cone2 _newpos_3 "0, 0, 0" false false 1.0 false))
    (:then_3
      (bind _newpos_4 (CallFunction|MoveDown _cone3))
      (Components|MoveComponentTo _cone3 _newpos_4 "0, 0, 0" false false 1.0 false)
      (Utilities|FlowControl|Delay (Math|Random|RandomFloatinRange 1.0 2.0))
      (CallFunction|Smash))))

(event EventBeginPlay
  (CallFunction|Smash))

(fn ConstructionScript)

(fn MoveDown
  (params (Static%20Mesh :type Static%20Mesh%20Component%20Object%20Reference))
  (bind _relativelocation (Variables|/Script/Engine.SceneComponent|GetRelativeLocation Static%20Mesh))
  (return (Math|Vector|MakeVector (.x _relativelocation) (.y _relativelocation) (* (.z (.Origin (Collision|GetComponentBounds Static%20Mesh))) -1.0))))

(fn MoveUp
  (params (Static%20Mesh :type Static%20Mesh%20Component%20Object%20Reference))
  (bind _relativelocation (Variables|/Script/Engine.SceneComponent|GetRelativeLocation Static%20Mesh))
  (return (Math|Vector|MakeVector (.x _relativelocation) (.y _relativelocation) (* (.z (.Origin (Collision|GetComponentBounds Static%20Mesh))) 1.0))))